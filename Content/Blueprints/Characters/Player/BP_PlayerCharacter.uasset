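; Player character Blueprint that sets up Enhanced Input and toggles the inventory widget.
; BeginPlay adds the mapping context, stores the cast HUD, then enters a shared add-inventory-to-viewport and Game-and-UI path.
; IA_OpenInventory flip-flops between creating the inventory into that path and removing it for Game-Only input, also reached by L after a delay.
; ShowLootToast creates a toast but joins the inventory path; toast display and cursor toggles are unconnected.
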(event Custom|ShowLootToast
  (bind _returnvalue (UserInterface|CreateWidget "/Game/Blueprints/UI/WBP_LootToast.WBP_LootToast_C"))
  (UserInterface|Viewport|AddtoViewport (stale Input|EnhancedActionEvents|EnhancedInputActionIA_OpenInventory _returnvalue_2) 0)
  (Input|SetInputModeGameandUI (Game|GetPlayerController 0) 0 "DoNotLock" false false))

(event Input|EnhancedActionEvents|EnhancedInputActionIA_OpenInventory
  (params (ActionValue :type Boolean) (ElapsedSeconds :type Float%20%28double-precision%29) (TriggeredSeconds :type Float%20%28double-precision%29) (InputAction :type Input%20Action%20Object%20Reference :default "/Game/Blueprints/Systems/Input/IA_OpenInventory.IA_OpenInventory"))
  (bind _returnvalue (Game|GetPlayerController 0))
  (Utilities|FlowControl|FlipFlop
    (:A
      (bind _returnvalue_2 (UserInterface|CreateWidget "/Game/Blueprints/UI/WBP_Inventory.WBP_Inventory_C"))
      (UserInterface|Viewport|AddtoViewport _returnvalue_2 0)
      (Input|SetInputModeGameandUI _returnvalue 0 "DoNotLock" false false))
    (:B
      (Widget|RemovefromParent _returnvalue_2)
      (Input|SetInputModeGameOnly _returnvalue false))))

(event EventBeginPlay
  (Input|AddMappingContext (PlayerController|LocalPlayerSubsystems|GetEnhancedInputLocalPlayerSubsystem) "/Game/Blueprints/Systems/Input/IMC_Player.IMC_Player" 0 "(bIgnoreAllPressedKeysUntilRelease=True,bForceImmediately=False,bNotifyUserSettings=False)")
  (bind _aswbp_hud (Utilities|Casting|CastToWBP_HUDClass))
  (Variables|Default|SetHUDWidget _aswbp_hud)
  (UserInterface|Viewport|AddtoViewport (stale Input|EnhancedActionEvents|EnhancedInputActionIA_OpenInventory _returnvalue_2) 0)
  (Input|SetInputModeGameandUI (Game|GetPlayerController 0) 0 "DoNotLock" false false))

(event Input|KeyboardEvents|L
  (params (Key :type Key%20Structure))
  (:Pressed
    (Utilities|FlowControl|Delay (Variables|Default|GetDuration))
    (Widget|RemovefromParent (stale Input|EnhancedActionEvents|EnhancedInputActionIA_OpenInventory _returnvalue_2))
    (Input|SetInputModeGameOnly (Game|GetPlayerController 0) false)))

(fn ConstructionScript)